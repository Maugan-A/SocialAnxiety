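; BP_Enemy_Doofus is a Hopper enemy that runs the BT_SimpleAI behavior tree and can be squashed by the player.
; A capsule hit from a player character with positive vertical velocity launches that player upward.
; It also disables the enemy's collision, stops its AI and flattens and lowers the sprite.
; A short timer then spawns a Niagara pop effect and destroys the enemy.
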(event `self.ReceiveBeginPlay`
  (bind _returnvalue (`AIBlueprintHelperLibrary.GetAIController` self))
  (`parent.ReceiveBeginPlay`)
  (`/Engine/EditorBlueprintResources/StandardMacros.IsValid` _returnvalue
    (:`Is Valid`
      (`AIController.RunBehaviorTree` _returnvalue "/Game/Hopper/AI/BT_SimpleAI.BT_SimpleAI"))))

(event `self.CapsuleComponent.OnComponentHit`
  (params (HitComponent :type "PrimitiveComponent Object Reference") (OtherActor :type "Actor Object Reference") (OtherComp :type "PrimitiveComponent Object Reference") (NormalImpulse :type "Vector Structure") (Hit :type "HitResult Structure (by ref)"))
  (bind _sprite (`self.Sprite`))
  (bind _returnvalue (`AIBlueprintHelperLibrary.GetAIController` self))
  (bind (_returnvalue_x _returnvalue_y _returnvalue_z) (`KismetMathLibrary.BreakVector` (`KismetMathLibrary.Normal` (`self.GetVelocity` OtherActor))))
  (bind (_relativescale3d_x _relativescale3d_y _relativescale3d_z) (`KismetMathLibrary.BreakVector` (`SceneComponent.RelativeScale3D` _sprite)))
  ;[0 0.2331 1] Squash
  (if (> _returnvalue_z 0.0)
    (bind _asbp_hopper_player_character (cast `/Game/Characters/MainCharacter/BP_HopperPlayerCharacter` OtherActor))
    (`self.LaunchCharacter` _asbp_hopper_player_character (0.0 0.0 400.0) false false)
    (`PrimitiveComponent.SetCollisionEnabled` (`self.CapsuleComponent`) "NoCollision")
    (`KismetSystemLibrary.PrintString` "Squashed!")
    (`Controller.StopMovement` _returnvalue)
    (`BrainComponent.StopLogic` (`AIController.BrainComponent` _returnvalue) "")
    (`SceneComponent.SetRelativeScale3D` _sprite (`KismetMathLibrary.MakeVector` _relativescale3d_x _relativescale3d_y (/ _relativescale3d_z 2.0)))
    (`SceneComponent.K2_AddLocalOffset` _sprite (0.0 0.0 -55.0) false true)
    (`KismetSystemLibrary.K2_SetTimerDelegate` (delegate `OnSquashed`) 1.0)))

(event `OnSquashed`
  (`NiagaraFunctionLibrary.SpawnSystemAtLocation` "/Game/Hopper/FX/N_Pop.N_Pop" (`self.K2_GetActorLocation`))
  (`self.K2_DestroyActor`))

(fn `UserConstructionScript`
  (`parent.UserConstructionScript`))