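; BP_DeadZone is a hazard volume that periodically damages the main character while it is inside.
; Box overlap events add and remove main characters in an ActorToDamage array.
; A looping one-second timer damages each listed actor and plays a camera shake at the player's location.
; The same loop shifts the zone itself along negative X, so it only moves while occupied.
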(event `self.ReceiveBeginPlay`
  (`KismetSystemLibrary.K2_SetTimerDelegate` (delegate `Damage Tick`) 1.0 true))

(event `Damage Tick`
  (bind (_returnvalue_x _returnvalue_y _returnvalue_z) (`KismetMathLibrary.BreakVector` (`self.K2_GetActorLocation`)))
  (for _array_element (`self.ActorToDamage`)
    (`GameplayStatics.ApplyDamage` _array_element (`self.Base Damage`))
    (`GameplayStatics.PlayWorldCameraShake` "/Game/Environment/Blueprints/BP_CameraShaker.BP_CameraShaker_C" (`self.K2_GetActorLocation` (`GameplayStatics.GetPlayerCharacter` 0)) 0.0 10000.0)
    (`self.K2_SetActorLocation` (`KismetMathLibrary.MakeVector` (- _returnvalue_x 150.0) _returnvalue_y _returnvalue_z))))

(event `self.Box.OnComponentBeginOverlap`
  (params (OverlappedComponent :type "PrimitiveComponent Object Reference") (OtherActor :type "Actor Object Reference") (OtherComp :type "PrimitiveComponent Object Reference") (OtherBodyIndex :type Integer) (bFromSweep :type Boolean) (SweepResult :type "HitResult Structure (by ref)"))
  (bind _asbp_main_character (cast `/Game/Characters/MainCharacter/BP_Main_character` OtherActor))
  (`/Engine/EditorBlueprintResources/StandardMacros.IsValid` _asbp_main_character
    (:`Is Valid`
      (`KismetArrayLibrary.Array_Add` (`self.ActorToDamage`) OtherActor))))

(event `self.Box.OnComponentEndOverlap`
  (params (OverlappedComponent :type "PrimitiveComponent Object Reference") (OtherActor :type "Actor Object Reference") (OtherComp :type "PrimitiveComponent Object Reference") (OtherBodyIndex :type Integer))
  (bind _returnvalue (`KismetArrayLibrary.Array_Find` (`self.ActorToDamage`) OtherActor))
  (if (>= _returnvalue 0)
    (`KismetArrayLibrary.Array_Remove` (`self.ActorToDamage`) _returnvalue)))

(fn `UserConstructionScript`)