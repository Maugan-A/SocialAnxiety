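; Wall actor that becomes passable once the player character's Facteur flag is true.
; BeginPlay applies the initial wall material to its cube and caches the BP_Main_character reference.
; Tick polls that flag, and a DoOnce then swaps the cube's material and disables its collision a single time, with no path back to solid.
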(event `self.ReceiveBeginPlay`
  (`PrimitiveComponent.SetMaterial` (`self.Cube`) 0 "/Game/Environment/House/Material/M_Wall2.M_Wall2")
  (bind _asbp_main_character (cast `/Game/Characters/MainCharacter/BP_Main_character` (`GameplayStatics.GetPlayerCharacter` 0)))
  (set `self.As BP Main Character` _asbp_main_character))

(event `self.ReceiveTick`
  (params (DeltaSeconds :type "Float (single-precision)"))
  (if (`/Game/Characters/MainCharacter/BP_Main_character.Facteur` (`self.As BP Main Character`))
    (`/Engine/EditorBlueprintResources/StandardMacros.DoOnce` false
      (:`Completed`
        (`PrimitiveComponent.SetMaterial` (`self.Cube`) 0 "/Game/Environment/House/Wall_2__1___1__Mat.Wall_2__1___1__Mat")
        (`PrimitiveComponent.SetCollisionEnabled` (`self.Cube`) "NoCollision")))))

(fn `UserConstructionScript`)