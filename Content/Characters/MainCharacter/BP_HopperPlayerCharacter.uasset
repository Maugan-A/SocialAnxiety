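; Player character for a sprite-based hopper, with a Mario-style triple jump, interaction and an energy meter.
; Landings within a short timer window step up jump power, while gravity increases at each apex and resets on landing.
; AttackRadius overlaps track one interactible, which the interact input messages before switching to UI-only input.
; Damage lowers Energy, which drives a post-process parameter collection alpha; debug keys alter time, delivery flag and energy.
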(event `self.ReceiveBeginPlay`
  (`parent.ReceiveBeginPlay`)
  (add `self.OnReachedJumpApex` (delegate `ModifyGravity`)))

(event `self.ReceiveTick`
  (params (DeltaSeconds :type "Float (single-precision)"))
  (`KismetMaterialLibrary.SetScalarParameterValue` "/Game/UI/PostProcess/PC_PP_Alpha.PC_PP_Alpha" "Alpha" (- 1.0 (/ (`self.Energy`) 100.0))))

(event `InputAction|Jump`
  (params (Key :type "Key Structure"))
  ;[1 0.685 0] Super Double Triple Jump
  (:`Pressed`
    (`self.Jump`)))

(event `self.OnJumped`
  ;[1 0.685 0] Super Double Triple Jump
  (set `CharacterMovementComponent.bNotifyApex` true (`self.CharacterMovement`))
  (`PaperFlipbookComponent.SetPlayRate` (`self.Sprite`) 0.0)
  (`PaperFlipbookComponent.SetPlaybackPositionInFrames` (`self.Sprite`) 0 true)
  (`/Engine/EditorBlueprintResources/StandardMacros.IncrementInt` (`self.JumpCounter`)
    (:`  `
      (`KismetSystemLibrary.K2_ClearAndInvalidateTimerHandle` (`self.JumpReset`)))))

(event `EnhancedInput|/Game/Core/Input/Actions/AI_Interact`
  (params (ActionValue :type Boolean) (ElapsedSeconds :type "Float (double-precision)") (TriggeredSeconds :type "Float (double-precision)") (InputAction :type "InputAction Object Reference" :default "/Game/Core/Input/Actions/AI_Interact.AI_Interact"))
  (:`Started`
    (`/Engine/EditorBlueprintResources/StandardMacros.IsValid` (`self.Interactible`) :!label _label
      (:`Is Valid`
        (message `/Game/Core/Dialogue_System/BP_Interactible.Interact` (`self.Interactible`) self)
        (`WidgetBlueprintLibrary.SetInputMode_UIOnlyEx` (`GameplayStatics.GetPlayerController` 0) null)
        (set `PlayerController.bShowMouseCursor` true (`GameplayStatics.GetPlayerController` 0))))))

(event `ModifyGravity`
  ;[1 0.685 0] Super Double Triple Jump
  ;;[1 1 1] at jump apex
  (set `CharacterMovementComponent.GravityScale` 5.0 (`self.CharacterMovement`)))

(event `Key|E`
  (params (Key :type "Key Structure"))
  (:`Pressed`
    (goto _label)))

(event `self.OnLanded`
  (params (Hit :type "HitResult Structure (by ref)"))
  ;[1 0.685 0] Super Double Triple Jump
  (`PaperFlipbookComponent.SetPlayRate` (`self.Sprite`) 1.0)
  (set `CharacterMovementComponent.GravityScale` 2.8 (`self.CharacterMovement`))
  (if (> (`self.JumpCounter`) 2)
    (set `self.JumpCounter` 0))
  (`self.ModifyJumpPower`)
  (bind _returnvalue (`KismetSystemLibrary.K2_SetTimerDelegate` (delegate `ResetJumpPower`) 0.2))
  (set `self.JumpReset` _returnvalue))

(event `self.AttackRadius.OnComponentBeginOverlap`
  (params (OverlappedComponent :type "PrimitiveComponent Object Reference") (OtherActor :type "Actor Object Reference") (OtherComp :type "PrimitiveComponent Object Reference") (OtherBodyIndex :type Integer) (bFromSweep :type Boolean) (SweepResult :type "HitResult Structure (by ref)"))
  (if (!= OtherActor self)
    (if (`KismetSystemLibrary.DoesImplementInterface` OtherActor "/Game/Core/Dialogue_System/BP_Interactible.BP_Interactible_C")
      (`/Engine/EditorBlueprintResources/StandardMacros.IsValid` (`self.Interactible`)
        (:`Is Valid`
          (message `/Game/Core/Dialogue_System/BP_Interactible.Set Interactible State` (`self.Interactible`) false)
          (set `self.Interactible` null))
        (:`Is Not Valid`
          _))
      (set `self.Interactible` OtherActor)
      (message `/Game/Core/Dialogue_System/BP_Interactible.Set Interactible State` (`self.Interactible`) true))))

(event `ModifyJumpPower`
  ;[1 0.685 0] Super Double Triple Jump
  (set `CharacterMovementComponent.JumpZVelocity` (select `int` (`self.JumpCounter`) :`0` 1200.0 :`1` 1400.0 :`2` 1800.0) (`self.CharacterMovement`)))

(event `self.AttackRadius.OnComponentEndOverlap`
  (params (OverlappedComponent :type "PrimitiveComponent Object Reference") (OtherActor :type "Actor Object Reference") (OtherComp :type "PrimitiveComponent Object Reference") (OtherBodyIndex :type Integer))
  (if (and (!= OtherActor self) (== OtherActor null))
    (message `/Game/Core/Dialogue_System/BP_Interactible.Set Interactible State` (`self.Interactible`) false)
    (set `self.Interactible` null)))

(event `ResetJumpPower`
  ;[1 0.685 0] Super Double Triple Jump
  (set `CharacterMovementComponent.JumpZVelocity` 1000.0 (`self.CharacterMovement`))
  (set `self.JumpCounter` 0))

(event `CustomEvent`
  (set `PlayerController.bShowMouseCursor` false (`GameplayStatics.GetPlayerController` 0))
  (`WidgetBlueprintLibrary.SetInputMode_GameOnly` (`GameplayStatics.GetPlayerController` 0)))

(event `Key|P`
  (params (Key :type "Key Structure"))
  (:`Pressed`
    (bind _output_get (set `self.Time of Day` (+ (`self.Time of Day`) (`KismetMathLibrary.MakeTimespan` 0 1))))
    (bind (_days _hours _minutes) (`KismetMathLibrary.BreakTimespan` _output_get))
    (`KismetSystemLibrary.PrintText` (`|FormatText` "{D}-{h}:{m}" _days _hours _minutes))))

(event `Key|M`
  (params (Key :type "Key Structure"))
  (:`Pressed`
    (set `self.Livraison?` true)))

(event `self.ReceiveAnyDamage`
  (params (Damage :type "Float (single-precision)") (DamageType :type "DamageType Object Reference") (InstigatedBy :type "Controller Object Reference") (DamageCauser :type "Actor Object Reference"))
  (set `self.Energy` (`KismetMathLibrary.FClamp` (- (`self.Energy`) Damage) 0.0 (`self.Max Energy`)))
  (if (== (`self.Energy`) 0.0)
    (`KismetSystemLibrary.PrintString` "PANIC")))

(event `Key|B`
  (params (Key :type "Key Structure"))
  (:`Pressed`
    (`GameplayStatics.ApplyDamage` self 20.0)))

(event `Key|N`
  (params (Key :type "Key Structure"))
  (:`Pressed`
    (`GameplayStatics.ApplyDamage` self -20.0)))

(fn `UserConstructionScript`)