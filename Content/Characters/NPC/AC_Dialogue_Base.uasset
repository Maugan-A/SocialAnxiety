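; Base NPC dialogue component that runs branching conversations through a UI_Dialogue widget, with optional voice audio.
; Each progression resets the index and replays the overridable Dialogue function; AddDialogue returns stored choices for answered steps, otherwise displaying the line.
; Selected options or auto-progress record choices in DialogueProgress, which BranchProgress stores per named branch.
; Audio plays on a runtime-created AudioComponent, async-loading unloaded soft references.
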(event `self.ReceiveBeginPlay`
  (if (`self.Use Audio?`)
    (bind _returnvalue (`|AddComponentByClass` :`self` (`self.GetOwner`) :`Class` "/Script/Engine.AudioComponent"))
    (set `self.Audio component` _returnvalue)))

(event `Load Dialogue audio`
  (params (`sound base` :type "SoundBase Soft Object Reference"))
  (bind _audio_component (`self.Audio component`))
  (bind _audio_component_2 (`self.Audio component`))
  (bind _object (`|LoadAsset` `sound base`)
    (:`Completed`
      (bind _assound_base (cast `SoundBase` _object))
      (`/Engine/EditorBlueprintResources/StandardMacros.IsValid` _audio_component_2
        (:`Is Valid`
          (`AudioComponent.SetSound` _audio_component_2 _assound_base)
          (`/Engine/EditorBlueprintResources/StandardMacros.IsValid` _audio_component
            (:`Is Valid`
              (`AudioComponent.Play` _audio_component 0.0))))))))

(fn `Add Dialogue`
  (params (Speaker :type Text) (Dialogue :type Text) (`Option Text` :type "Array of Text") (`Dialogue Audio ` :type "SoundBase Soft Object Reference"))
  (returns (State :type "/Game/Core/Dialogue_System/Enum_Progress_Dialogue_State Enum") (`Option Index` :type Integer))
  (bind (_value _returnvalue) (`BlueprintMapLibrary.Map_Find` (`self.DialogueProgress`) (`self.DialogueIndex`)))
  (`/Engine/EditorBlueprintResources/StandardMacros.IncrementInt` (`self.DialogueIndex`)
    (:`  `
      (if _returnvalue
        (return "NewEnumerator0" _value)
        (else
          (`/Game/UI/UI_Dialogue.UpdateDialogueText` (`self.DialogueWidget`) (`self.DialogueIndex`) (`local.Speaker`) (`local.Dialogue`) (`local.Option Text`))
          (`self.Play Dialogue Audio` (`local.Dialogue Audio `))
          (return "NewEnumerator1" 0))))))

(fn `Auto Progress`
  (`self.Update Selected Option` (`self.DialogueIndex`)))

(fn `Clear Dialogue Progress`
  (`BlueprintMapLibrary.Map_Clear` (`self.DialogueProgress`)))

(fn `Close Conversation`
  (`Widget.RemoveFromParent` (`self.DialogueWidget`))
  (bind _audio_component (`self.Audio component`)
    (:`then`
      (`AudioComponent.Stop` _audio_component))
    (:`else`
      _))
  (message `/Game/Core/Dialogue_System/BP_Interactible.Conversation Closed` (`self.GetOwner`)))

(fn `Dialogue`)

(fn `NewFunction`)

(fn `OpenConversation`
  (bind _returnvalue (`|CreateWidget` "/Game/UI/UI_Dialogue.UI_Dialogue_C" null self))
  (set `self.DialogueWidget` _returnvalue)
  (add `/Game/UI/UI_Dialogue.OnAutoProgress` (`self.DialogueWidget`) (`|CreateDelegate` :!event `Auto Progress`))
  (`UserWidget.AddToViewport` (`self.DialogueWidget`) 0)
  (`self.Progress Dialogue`))

(fn `Play Dialogue Audio`
  (params (Audio :type "SoundBase Soft Object Reference (by ref)"))
  (bind _audio_component (`self.Audio component`))
  (bind _audio_component_2 (`self.Audio component`))
  (bind _output (`|ConvertAsset` (`local.Audio`)))
  (if (and (`KismetSystemLibrary.IsValidSoftObjectReference` Audio) (`self.Use Audio?`))
    (`/Engine/EditorBlueprintResources/StandardMacros.IsValid` _output
      (:`Is Valid`
        (`/Engine/EditorBlueprintResources/StandardMacros.IsValid` _audio_component
          (:`Is Valid`
            (`AudioComponent.SetSound` _audio_component _output)
            (`/Engine/EditorBlueprintResources/StandardMacros.IsValid` _audio_component_2
              (:`Is Valid`
                (`AudioComponent.Play` _audio_component_2 0.0))))))
      (:`Is Not Valid`
        (`self.Load Dialogue audio` (`local.Audio`))))))

(fn `Progress Dialogue`
  (set `self.DialogueIndex` -4)
  (`self.Dialogue`))

(fn `Remove Dialogue Progress`
  (params (`Progress Steps` :type Integer))
  (for _index (range (+ `Progress Steps` 1))
    (`BlueprintMapLibrary.Map_Remove` (`self.DialogueProgress`) (- (`self.DialogueIndex`) _index))))

(fn `Set dialogue Branch`
  (params (`Dialogue Branch` :type Name) (ProgressHandler :type "/Game/Core/Dialogue_System/Enum_Dialogue_ProgressStoreType Enum" :default "NewEnumerator0"))
  (switch `/Game/Core/Dialogue_System/Enum_Dialogue_ProgressStoreType` ProgressHandler
    (:`NewEnumerator0`
      (`BlueprintMapLibrary.Map_Add` (`self.BranchProgress`) (`self.ActiveDialogueBranch`) (make `/Game/Core/Dialogue_System/Structure_Dialogue_Progress` (`self.DialogueProgress`))))
    (:`NewEnumerator1`
      (`BlueprintMapLibrary.Map_Add` (`self.BranchProgress`) (`self.ActiveDialogueBranch`))))
  (set `self.DialogueProgress` (break `/Game/Core/Dialogue_System/Structure_Dialogue_Progress` (`BlueprintMapLibrary.Map_Find` (`self.BranchProgress`) (`self.ActiveDialogueBranch`))))
  (set `self.ActiveDialogueBranch` (`local.Dialogue Branch`)))

(fn `Update Selected Option`
  (params (`Progress Index` :type Integer) (`Option Index` :type "Integer (by ref)"))
  (`BlueprintMapLibrary.Map_Add` (`self.DialogueProgress`) `Progress Index` `Option Index`)
  (`self.Progress Dialogue`))