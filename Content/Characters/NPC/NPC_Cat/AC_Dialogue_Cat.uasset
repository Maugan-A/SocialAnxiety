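; Dialogue component for the cat NPC Nana, who meows through a French-language branching conversation with the player.
; The default branch offers nested choices; petting her saves the Pet_ok branch, switches the owner's Paper2D flipbook to sleeping and applies negative damage to the player, presumably as healing.
; Once that branch is active, later talks only play one of several random sleepy lines.
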(event `self.ReceiveBeginPlay`
  (bind _asbp_main_character (cast `/Game/Characters/MainCharacter/BP_Main_character` (`GameplayStatics.GetPlayerCharacter` 0)))
  (set `self.As BP Main Character` _asbp_main_character))

(fn `Dialogue`
  (`parent.Dialogue`)
  (switch `name` (`self.ActiveDialogueBranch`)
    (:`Default`
      (bind (_state _option_index) (`self.Add Dialogue` "Nana" "Miaou?" (`|MakeArray` "Oui pas de soucis." "Non désolé." :!type "Text") "/Game/Sounds/cat-meow-14536.cat-meow-14536"))
      (switch `/Game/Core/Dialogue_System/Enum_Progress_Dialogue_State` _state
        (:`NewEnumerator0`
          (switch `int` _option_index
            (:`0`
              (bind (_state_2 _option_index_2) (`self.Add Dialogue` "Nana" "Miaou ! Miaou..." (`|MakeArray` "[Caresser Nana]" "[Partir]" :!type "Text") "/Game/Sounds/cat-meow-14536.cat-meow-14536"))
              (switch `/Game/Core/Dialogue_System/Enum_Progress_Dialogue_State` _state_2
                (:`NewEnumerator0`
                  (switch `int` _option_index_2
                    (:`0`
                      (bind _state_3 (`self.Add Dialogue` :`Speaker` "Nana" :`Dialogue` "Miaou !" :`Dialogue Audio ` "/Game/Sounds/cat-meow-14536.cat-meow-14536"))
                      (switch `/Game/Core/Dialogue_System/Enum_Progress_Dialogue_State` _state_3
                        (:`NewEnumerator0`
                          (`|ExecutionSequence`
                            (:`then_0`
                              (`self.Set dialogue Branch` "Pet_ok")
                              (`self.Clear Dialogue Progress`)
                              (`self.Close Conversation`)
                              (`PaperFlipbookComponent.SetFlipbook` (`Actor.GetComponentByClass` (`self.GetOwner`) "/Script/Paper2D.PaperFlipbookComponent") "/Game/Characters/NPC/NPC_Cat/Animation/Cat_Sleep_Frame10.Cat_Sleep_Frame10"))
                            (:`then_1`
                              (`GameplayStatics.ApplyDamage` (`self.As BP Main Character`) -40.0))))))
                    (:`1`
                      (bind _state_4 (`self.Add Dialogue` :`Speaker` "Nana" :`Dialogue` "Miaou." :`Dialogue Audio ` "/Game/Sounds/cat-meow-14536.cat-meow-14536"))
                      (switch `/Game/Core/Dialogue_System/Enum_Progress_Dialogue_State` _state_4
                        (:`NewEnumerator0`
                          (`self.Remove Dialogue Progress` 2)
                          (`self.Close Conversation`))))))))
            (:`1`
              (bind _state_5 (`self.Add Dialogue` :`Speaker` "Nana" :`Dialogue` "Mia...ou?" :`Dialogue Audio ` "/Game/Sounds/cat-meow-14536.cat-meow-14536"))
              (switch `/Game/Core/Dialogue_System/Enum_Progress_Dialogue_State` _state_5
                (:`NewEnumerator0`
                  (`self.Clear Dialogue Progress`)
                  (`self.Close Conversation`))))))))
    (:`Pet_ok`
      (bind _state_6 (`self.Add Dialogue` :`Speaker` "Nana" :`Dialogue` (select `int` (`KismetMathLibrary.RandomIntegerInRange` 0 2) :`0` "zZz..." :`1` "zZz... miaou..zZz..." :`2` "zZz..miaou...?" :!type "Text") :`Dialogue Audio ` "/Game/Sounds/cat-meow-14536.cat-meow-14536"))
      (switch `/Game/Core/Dialogue_System/Enum_Progress_Dialogue_State` _state_6
        (:`NewEnumerator0`
          (`self.Clear Dialogue Progress`)
          (`self.Close Conversation`))))))