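; Dialogue component for the postman NPC (Facteur), extending a parent branching-dialogue system with French lines.
; On opening, it records whether the player's Key flag is set as Docs and picks a Night, Morning or Afternoon branch from the hour.
; Only Night is wired, playing a random demo placeholder line before closing.
; Other greetings and a parcel-pickup exchange, which checks Docs and reveals BP_Colis, are present but disconnected.
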(fn `Dialogue`
  (`parent.Dialogue`)
  (switch `name` (`self.ActiveDialogueBranch`)
    (:`Night`
      (bind _state (`self.Add Dialogue` "Facteur" (select `int` (`KismetMathLibrary.RandomIntegerInRange` 0 4) :`0` "C'est tout pour cette démo !" :`1` "C'est tout pour le moment." :`2` "Mes dialogues sont encore en cours d'écriture." :`3` "Alt + F4 pour quitter." :`4` "Attendez.. Je vous connais !" :!type "Text")))
      (switch `/Game/Core/Dialogue_System/Enum_Progress_Dialogue_State` _state
        (:`NewEnumerator0`
          (`self.Clear Dialogue Progress`)
          (`self.Close Conversation`))))))

(fn `OpenConversation`
  (bind _interaction_instigator (message `/Game/Core/Dialogue_System/BP_Interactible.Get Interaction Instigator` (`self.GetOwner`)))
  (bind _asbp_main_character (cast `/Game/Characters/MainCharacter/BP_Main_character` _interaction_instigator))
  (if (`/Game/Characters/MainCharacter/BP_Main_character.Key?` _asbp_main_character)
    (set `self.Docs?` true)
    (else
      (set `self.Docs?` false)))
  (bind (_time_of_day_days _time_of_day_hours) (`KismetMathLibrary.BreakTimespan` (`/Game/Characters/MainCharacter/BP_Main_character.Time of Day` _asbp_main_character)))
  (`self.Set dialogue Branch` (select `int` (+ (`KismetMathLibrary.Conv_BoolToInt` (and (>= _time_of_day_hours 5) (< _time_of_day_hours 12))) (* (`KismetMathLibrary.Conv_BoolToInt` (and (>= _time_of_day_hours 13) (< _time_of_day_hours 22))) 2)) :`0` "Night" :`1` "Morning" :`2` "Afternoon" :`3` "Default" :!type "Name"))
  (`parent.OpenConversation`))