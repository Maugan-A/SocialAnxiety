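; Dialogue component for an in-game computer that shows a French-language inbox where the player can reschedule a postal delivery.
; It overrides the parent dialogue system's Dialogue function as a branching tree, with options gated by the main character's Energy cached at BeginPlay.
; Rescheduling spends energy via ApplyDamage, sets the character's Livraison flag and switches to a branch reporting no new messages.
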(event `self.ReceiveBeginPlay`
  (`parent.ReceiveBeginPlay`)
  (bind _asbp_main_character (cast `/Game/Characters/MainCharacter/BP_Main_character` (`GameplayStatics.GetPlayerCharacter` 0)))
  (set `self.As BP Main Character` _asbp_main_character))

(fn `Dialogue`
  (`parent.Dialogue`)
  (switch `name` (`self.ActiveDialogueBranch`)
    (:`Default`
      (bind (_state _option_index) (`self.Add Dialogue` "Ordinateur" "Vous avez [1] nouveaux message ! " (`|MakeArray` "[BureauPostal.com]" "[Quitter]" :!type "Text")))
      (switch `/Game/Core/Dialogue_System/Enum_Progress_Dialogue_State` _state
        (:`NewEnumerator0`
          (switch `int` _option_index
            (:`0`
              (bind (_state_2 _option_index_2) (`self.Add Dialogue` "BureauPostal.com" "Vous avez une livraison à reprogrammer !" (select `bool` (> (`/Game/Characters/MainCharacter/BP_Main_character.Energy` (`self.As BP Main Character`)) 20.0) :`false` (`|MakeArray` "Je n'ai pas l'énergie pour ça, on verra plus tard..." :!type "Text") :`true` (`|MakeArray` "On verra plus tard..." "Reprogrammer maintenant. [-1 Energie]" :!type "Text"))))
              (switch `/Game/Core/Dialogue_System/Enum_Progress_Dialogue_State` _state_2
                (:`NewEnumerator0`
                  (switch `int` _option_index_2
                    (:`0`
                      (bind _state_3 (`self.Add Dialogue` "Ordinateur" "A bientôt !"))
                      (switch `/Game/Core/Dialogue_System/Enum_Progress_Dialogue_State` _state_3
                        (:`NewEnumerator0`
                          (`self.Remove Dialogue Progress` 2)
                          (`self.Close Conversation`))))
                    (:`1`
                      (bind _state_4 (`self.Add Dialogue` "BureauPostal.com" "Très bien ! Un de nos facteur sera bientôt chez vous."))
                      (switch `/Game/Core/Dialogue_System/Enum_Progress_Dialogue_State` _state_4
                        (:`NewEnumerator0`
                          (`GameplayStatics.ApplyDamage` (`self.As BP Main Character`) 20.0)
                          (`self.Set dialogue Branch` "No message")
                          (`self.Clear Dialogue Progress`)
                          (`self.Close Conversation`)
                          (set `/Game/Characters/MainCharacter/BP_Main_character.Livraison?` true (`self.As BP Main Character`)))))))))
            (:`1`
              (bind _state_5 (`self.Add Dialogue` "Ordinateur !" "A bientôt !"))
              (switch `/Game/Core/Dialogue_System/Enum_Progress_Dialogue_State` _state_5
                (:`NewEnumerator0`
                  (`self.Remove Dialogue Progress` 1)
                  (`self.Close Conversation`))))))))
    (:`No message`
      (bind _state_6 (`self.Add Dialogue` "Ordinateur" "Pas de nouveaux message."))
      (switch `/Game/Core/Dialogue_System/Enum_Progress_Dialogue_State` _state_6
        (:`NewEnumerator0`
          (`self.Clear Dialogue Progress`)
          (`self.Close Conversation`))))))