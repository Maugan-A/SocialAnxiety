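; Bed dialogue component that lets the player's character comment on fatigue or rest, with French text.
; Tick switches the branch to EnergyLow when the main character's Energy is 50 or below, otherwise Default.
; Default plays a random one-liner, while EnergyLow offers a rest choice.
; Resting applies negative damage, presumably to restore energy, then closes the conversation and sets NewDay on the character.
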(event `self.ReceiveTick`
  (params (DeltaSeconds :type "Float (single-precision)"))
  (if (<= (`/Game/Characters/MainCharacter/BP_Main_character.Energy` (`self.As BP Main Character`)) 50.0)
    (`self.Set dialogue Branch` "EnergyLow")
    (else
      (`self.Set dialogue Branch` "Default"))))

(event `self.ReceiveBeginPlay`
  (bind _asbp_main_character (cast `/Game/Characters/MainCharacter/BP_Main_character` (`GameplayStatics.GetPlayerCharacter` 0)))
  (set `self.As BP Main Character` _asbp_main_character))

(fn `Dialogue`
  (`parent.Dialogue`)
  (switch `name` (`self.ActiveDialogueBranch`)
    (:`Default`
      (bind _state (`self.Add Dialogue` "Vous" (select `int` (`KismetMathLibrary.RandomIntegerInRange` 0 2) :`0` "Je ne suis pas fatigué." :`1` "Aller, courage pour cette journée !" :`2` "Vivement ce soir que je me recouche." :!type "Text")))
      (switch `/Game/Core/Dialogue_System/Enum_Progress_Dialogue_State` _state
        (:`NewEnumerator0`
          (`self.Clear Dialogue Progress`)
          (`self.Close Conversation`))))
    (:`EnergyLow`
      (bind (_state_2 _option_index) (`self.Add Dialogue` "Vous" "Je suis épuisée, je devrais peut être me reposer..." (`|MakeArray` "[Se Reposer] +4 Energie" "J'ai encore des choses à faire." :!type "Text")))
      (switch `/Game/Core/Dialogue_System/Enum_Progress_Dialogue_State` _state_2
        (:`NewEnumerator0`
          (switch `int` _option_index
            (:`0`
              (bind _state_3 (`self.Add Dialogue` "Vous" "zZz..."))
              (switch `/Game/Core/Dialogue_System/Enum_Progress_Dialogue_State` _state_3
                (:`NewEnumerator0`
                  (`GameplayStatics.ApplyDamage` (`self.As BP Main Character`) -60.0)
                  (`self.Remove Dialogue Progress` 2)
                  (`self.Close Conversation`)
                  (set `/Game/Characters/MainCharacter/BP_Main_character.New Day?` true (`self.As BP Main Character`)))))
            (:`1`
              (`self.Clear Dialogue Progress`)
              (`self.Close Conversation`))))))))