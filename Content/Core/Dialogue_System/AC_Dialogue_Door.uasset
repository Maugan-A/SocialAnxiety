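; Door dialogue component that lets the player either answer the postman's delivery or hear a random refusal to go out.
; Tick watches the main character's Livraison and NewDay flags to switch between delivery and closed-door branches, with DoOnce gates re-armed on a new day.
; Opening the door plays the postman's greeting, sets the player's Facteur flag and applies negative damage to the player, on an option labelled as costing energy.
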(event `self.ReceiveTick`
  (params (DeltaSeconds :type "Float (single-precision)"))
  (bind _as_bp_main_character (`self.As BP Main Character`))
  (`|ExecutionSequence`
    (:`then_0`
      (if (`/Game/Characters/MainCharacter/BP_Main_character.Livraison?` _as_bp_main_character)
        (`/Engine/EditorBlueprintResources/StandardMacros.DoOnce` false :!label _label
          (:`Completed`
            (`self.Set dialogue Branch` "Livraison")))))
    (:`then_1`
      (if (`/Game/Characters/MainCharacter/BP_Main_character.New Day?` _as_bp_main_character)
        (`/Engine/EditorBlueprintResources/StandardMacros.DoOnce` false :!label _label_2
          (:`Completed`
            (`self.Set dialogue Branch` "PorteFermée")
            (`TypedElementListLibrary.Reset` (struct))))))))

(event `Reset`
  (`|ExecutionSequence`
    (:`then_0`
      (goto _label :!via `Reset`))
    (:`then_1`
      (goto _label_2 :!via `Reset`))))

(event `self.ReceiveBeginPlay`
  (bind _asbp_main_character (cast `/Game/Characters/MainCharacter/BP_Main_character` (`GameplayStatics.GetPlayerCharacter` 0)))
  (set `self.As BP Main Character` _asbp_main_character)
  (`self.Set dialogue Branch` "PorteFermée"))

(fn `Dialogue`
  (`parent.Dialogue`)
  (switch `name` (`self.ActiveDialogueBranch`)
    (:`Livraison`
      (bind (_state _option_index) (`self.Add Dialogue` "Vous" "" (select `bool` false :`false` (`|MakeArray` "Non tant pis, il repassera plus tard de toutes façons." "[Ouvrir la porte] -1 Energie." :!type "Text") :`true` (`|MakeArray` "Non tant pis, il repassera plus tard de toutes façons." :!type "Text"))))
      (switch `/Game/Core/Dialogue_System/Enum_Progress_Dialogue_State` _state
        (:`NewEnumerator0`
          (switch `int` _option_index
            (:`0`
              (`self.Clear Dialogue Progress`)
              (`self.Close Conversation`))
            (:`1`
              (bind _state_2 (`self.Add Dialogue` :`Speaker` "Facteur" :`Dialogue` "Bonjour, bonjour !" :`Dialogue Audio ` "/Game/Sounds/cat-meow-14536.cat-meow-14536"))
              (switch `/Game/Core/Dialogue_System/Enum_Progress_Dialogue_State` _state_2
                (:`NewEnumerator0`
                  (`|ExecutionSequence`
                    (:`then_0`
                      (`self.Clear Dialogue Progress`)
                      (`self.Close Conversation`)
                      (set `/Game/Characters/MainCharacter/BP_Main_character.Facteur` true (`self.As BP Main Character`)))
                    (:`then_1`
                      (`GameplayStatics.ApplyDamage` (`self.As BP Main Character`) -20.0))))))))))
    (:`PorteFermée`
      (bind _state_3 (`self.Add Dialogue` "Vous" (select `int` (`KismetMathLibrary.RandomIntegerInRange` 0 2) :`0` "Je n'ai rien à faire dehors." :`1` "Je devrais m'occuper de cette livraison..." :`2` "Non je n'ai pas envie de sortir." :!type "Text")))
      (switch `/Game/Core/Dialogue_System/Enum_Progress_Dialogue_State` _state_3
        (:`NewEnumerator0`
          (`self.Clear Dialogue Progress`)
          (`self.Close Conversation`))))))